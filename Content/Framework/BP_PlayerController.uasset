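; BP_PlayerController is a player controller for cursor-driven movement and orb spawning.
; While PrimaryAction is held, an open Gate passes Tick through to add movement input toward the point under the cursor, found by a complex Visibility trace.
; Releasing the action closes the Gate.
; Pressing SpawnOrb spawns a BP_Orb at the controlled pawn's location.
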(event EventTick
  (params (DeltaSeconds :type Float%20%28single-precision%29))
  (bind _returnvalue (Pawn|GetControlledPawn))
  (Utilities|FlowControl|Gate true
    (:Exit
      (Pawn|Input|AddMovementInput _returnvalue (Math|Vector|GetUnitDirection(Vector) (Transformation|GetActorLocation _returnvalue) (.Location (Collision|BreakHitResult (.HitResult (Game|Player|GetHitResultUnderCursorbyChannel "TraceTypeQuery1" true))))) 1.0 false))))

(event Input|ActionEvents|InputActionSpawnOrb
  (params (Key :type Key%20Structure :default "None"))
  (:Pressed
    (Game|SpawnActorfromClass "/Game/GameElements/BP_Orb.BP_Orb_C" (Math|Transform|MakeTransform (Transformation|GetActorLocation (Pawn|GetControlledPawn)) "0, 0, 0" "1.000000,1.000000,1.000000") "Undefined" 0 0)))

(event Input|ActionEvents|InputActionPrimaryAction
  (params (Key :type Key%20Structure :default "None"))
  (bind _returnvalue (Pawn|GetControlledPawn))
  (:Pressed
    (Utilities|FlowControl|Gate true) ; enters at Open
  )
  (:Released
    (Utilities|FlowControl|Gate true) ; enters at Close
  ))

(fn ConstructionScript)