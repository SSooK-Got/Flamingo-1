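; BP_Door is a door actor that opens and closes when its assigned Trigger reports an interaction.
; On BeginPlay it binds to the Trigger's BP_InteractionComponent, and the On flag plays or reverses a single timeline.
; The timeline slides both door meshes along relative Y and fires a world camera shake at the door's location on each update.
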(event Custom|CloseDoor
  (bind _prog (Timeline|Timeline Reverse)
    (:Update
      (Transformation|SetRelativeLocation (Variables|Default|GetSM_Door_L) (Math|Vector|MakeVector 0.0 (* _prog -7e+01) 0.0) false false)
      (Camera|PlayWorldCameraShake "/Game/Effects/CameraShake.CameraShake_C" (Transformation|GetActorLocation) 0.0 1e+05))))

(event Custom|OpenDoor
  (bind _prog (Timeline|Timeline Play)
    (:Update
      (Transformation|SetRelativeLocation (Variables|Default|GetSM_Door_L) (Math|Vector|MakeVector 0.0 (* _prog -7e+01) 0.0) false false)
      (Camera|PlayWorldCameraShake "/Game/Effects/CameraShake.CameraShake_C" (Transformation|GetActorLocation) 0.0 1e+05))))

(event Custom|OnInteraction_Event
  (params (On :type Boolean))
  (if On
    (CallFunction|OpenDoor)
    (else
      (CallFunction|CloseDoor))))

(event EventBeginPlay
  (bind _trigger (Variables|Default|GetTrigger)
    (:then
      (Utilities|IsValid (Actor|GetComponentbyClass _trigger "/Game/Framework/BP_InteractionComponent.BP_InteractionComponent_C")
        (:Is%20Valid
          (EventDispatchers|AssignOnInteraction (Actor|GetComponentbyClass _trigger "/Game/Framework/BP_InteractionComponent.BP_InteractionComponent_C") (delegate Custom|OnInteraction_Event)))))
    (:else)))

(fn ConstructionScript)